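; Elevator actor that moves a cabin vertically between preset floor heights in response to cabin and call buttons.
; Its construction script spawns one cabin button per floor as a child actor.
; A floor request closes the doors; the child doors' closed event starts fixed-step, per-tick movement without delta-time scaling.
; On arrival it snaps to the target height and opens child and destination-floor doors, which auto-close on a timer.
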(event Custom|GoToFloor
  (params (FloorIndex :type Integer))
  (Variables|Default|SetWhichFloorDoors FloorIndex)
  (Variables|Default|SetFinish (Utilities|Array|Get(acopy) (Variables|Lift|GetFloors) FloorIndex))
  (CallFunction|SetupSign)
  ;[1 1 1] Закрытие дверей после нажатия кнопки
  (Default|CloseDoors (Variables|Lift|GetDoors) false)
  (Default|CloseDoors (Variables|Default|GetAs%20BP%20Floor%20Doors) true))

(event Custom|OnClosed
  (Variables|Default|SetIsMoving true))

(event Custom|AutoClose
  ;[1 1 1] Автоматическое закрытие дверей
  (Default|CloseDoors (Variables|Lift|GetDoors) false)
  (Default|CloseDoors (Variables|Default|GetAs%20BP%20Floor%20Doors) false))

(event Custom|OnOpened
  (Utilities|Time|SetTimerbyEvent (delegate Custom|AutoClose) 5.0))

(event EventBeginPlay
  (bind _asbp_floor_doors (Utilities|Casting|CastToBP_FloorDoors (Variables|/Script/Engine.ChildActorComponent|GetChildActor (Variables|Default|GetDoorsParent))))
  (Variables|Default|SetAs%20BP%20Floor%20Doors _asbp_floor_doors)
  (EventDispatchers|BindEventtoOnOpened (Variables|Default|GetAs%20BP%20Floor%20Doors) (delegate Custom|OnOpened))
  (EventDispatchers|BindEventtoOnClosed (Variables|Default|GetAs%20BP%20Floor%20Doors) (delegate Custom|OnClosed))
  (for _array_element (Variables|Default|GetElevatorButtons)
    (EventDispatchers|BindEventtoOnGotoFloor _array_element (delegate Custom|GoToFloor)))
  (for _array_element_2 (Variables|Lift|GetCallButtons)
    (EventDispatchers|BindEventtoOnGotoFloor _array_element_2 (delegate Custom|GoToFloor))))

(event EventTick
  (params (DeltaSeconds :type Float%20%28single-precision%29))
  (if (Variables|Default|GetIsMoving)
    (CallFunction|MovementProcess)))

(fn ConstructionScript
  (for (_ _array_index) (Variables|Lift|GetFloors)
    (bind _returnvalue (CallFunction|CreateButton _array_index))
    (Variables|/Game/Blueprints/BP_LiftButton.BP_LiftButton_C|SetFloor _returnvalue _array_index)
    (Utilities|Array|Add (Variables|Default|GetElevatorButtons) _returnvalue)))

(fn SetupSign
  (Variables|Default|SetSign (Math|Float|Sign(Float) (- (Variables|Default|GetFinish) (Variables|Default|GetCurrentHeight)))))

(fn IsNextPositionNotFinish
  (return (< (* (- (+ (Variables|Default|GetCurrentHeight) (* (Variables|Lift|GetMoveSpeed) (Variables|Default|GetSign))) (Variables|Default|GetFinish)) (Variables|Default|GetSign)) 0.0)))

(fn SetHight
  (params (Height :type Float%20%28double-precision%29))
  (bind _output_get (Variables|Default|SetCurrentHeight Height))
  (Transformation|SetRelativeLocation (Variables|Default|GetLift_FBX1) (Math|Vector|MakeVector 0.0 0.0 _output_get) false false))

(fn MovementProcess
  (if (CallFunction|IsNextPositionNotFinish)
    (CallFunction|SetHight (+ (Variables|Default|GetCurrentHeight) (* (Variables|Lift|GetMoveSpeed) (Variables|Default|GetSign))))
    (else
      (CallFunction|SetHight (Variables|Default|GetFinish))
      (Variables|Default|SetIsMoving false)
      (Default|OpenDoors (Utilities|Array|Get(acopy) (Variables|Lift|GetDoors) (Variables|Default|GetWhichFloorDoors)) false)
      (Default|OpenDoors (Variables|Default|GetAs%20BP%20Floor%20Doors) true))))

(fn CreateButton
  (params (Index :type Integer))
  (bind _returnvalue (AddComponent|AddChildActorComponent true))
  (Transformation|AttachComponentToComponent _returnvalue (Variables|Default|GetButtonsParent) "None" "SnapToTarget" "SnapToTarget" "KeepWorld" false)
  (Transformation|SetRelativeLocation _returnvalue (CallFunction|GetButtonLocation Index) false false)
  (ChildActorComponent|SetChildActorClass _returnvalue "/Game/Blueprints/BP_LiftButton.BP_LiftButton_C")
  (bind _asbp_lift_button (Utilities|Casting|CastToBP_LiftButton (Variables|/Script/Engine.ChildActorComponent|GetChildActor _returnvalue)))
  (return _asbp_lift_button))

(fn GetButtonLocation
  (params (Index :type Integer))
  (return (Math|Vector|MakeVector 0.0 (Math|Conversions|ToFloat(Integer) (* Index -80)) 0.0)))