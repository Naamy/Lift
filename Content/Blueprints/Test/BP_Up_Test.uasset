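; Test actor that moves its Cube vertically from a starting Height to a Finish height once its Button is pressed.
; The construction script applies Height to the Cube, and BeginPlay binds the button event and derives the travel direction from the sign of the distance.
; After the press, Tick steps by MoveSpeed without delta-time scaling, using a signed comparison to clamp at Finish in either direction.
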(event Custom|start
  (Variables|Default|SetisPressed true))

(event EventBeginPlay
  (EventDispatchers|BindEventtoOnPressed (Variables|Default|Getbutton) (delegate Custom|start))
  (CallFunction|SetupSign))

(event EventTick
  (params (DeltaSeconds :type Float%20%28single-precision%29))
  (if (Variables|Default|GetisPressed)
    (CallFunction|MovementProcess)))

(fn ConstructionScript
  (CallFunction|SetHeight (Variables|Default|GetHeight)))

(fn SetHeight
  (params (Height :type Float%20%28single-precision%29))
  (bind _output_get (Variables|Default|SetHeight Height))
  (Transformation|SetRelativeLocation (Variables|Default|GetCube) (Math|Vector|MakeVector 0.0 0.0 _output_get) false false))

(fn IsNextPositionLower
  (return (<= (* (- (+ (Variables|Default|GetHeight) (* (Variables|Default|GetmoveSpeed) (Variables|Default|GetSign))) (Variables|Default|Getfinish)) (Variables|Default|GetSign)) 0.0)))

(fn SetupSign
  (Variables|Default|SetSign (Math|Float|Sign(Float) (- (Variables|Default|Getfinish) (Variables|Default|GetHeight)))))

(fn MovementProcess
  (if (CallFunction|IsNextPositionLower)
    (CallFunction|SetHeight (+ (Variables|Default|GetHeight) (* (Variables|Default|GetmoveSpeed) (Variables|Default|GetSign))))
    (else
      (CallFunction|SetHeight (Variables|Default|Getfinish)))))