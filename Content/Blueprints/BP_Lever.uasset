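; BP_Lever is an interactable lever that shows an interact prompt while the first-person character stands inside its CallCollision volume.
; Overlap begin creates an InteractWidget on screen, and overlap end removes it.
; Activate plays a timeline that pitches the cylinder handle and fires the OnPressed dispatcher for other objects to respond to.
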(event OnComponentBeginOverlap(CallCollision)
  (params (OverlappedComponent :type Primitive%20Component%20Object%20Reference) (OtherActor :type Actor%20Object%20Reference) (OtherComp :type Primitive%20Component%20Object%20Reference) (OtherBodyIndex :type Integer) (bFromSweep :type Boolean) (SweepResult :type Hit%20Result%20Structure%20%28by%20ref%29))
  (Utilities|Casting|CastToFirstPersonCharacter OtherActor)
  (bind _returnvalue (UserInterface|CreateWidget (Variables|Default|GetInteractWidget)))
  (UserInterface|Viewport|AddtoViewport _returnvalue 0))

(event OnComponentEndOverlap(CallCollision)
  (params (OverlappedComponent :type Primitive%20Component%20Object%20Reference) (OtherActor :type Actor%20Object%20Reference) (OtherComp :type Primitive%20Component%20Object%20Reference) (OtherBodyIndex :type Integer))
  (Utilities|Casting|CastToFirstPersonCharacter OtherActor)
  (Widget|RemovefromParent (stale OnComponentBeginOverlap(CallCollision) _returnvalue)))

(event Custom|AnimateButton
  (bind _rotation (Timeline|lever PlayFromStart)
    (:Update
      (Transformation|SetWorldRotation (Variables|Default|GetCylinder) (Math|Rotator|MakeRotator 0.0 _rotation 9e+01) false false))))

(fn ConstructionScript)

(fn Activate
  (CallFunction|AnimateButton)
  (Default|CallOnPressed)
  (return))