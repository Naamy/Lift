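; BP_FloorDoors is a pair of sliding floor doors that open and close on request.
; OpenDoors and CloseDoors check an IsClosed flag, then play a shared timeline forward from the start or in reverse from the end.
; The timeline's LeftDoor and RightDoor tracks drive helper functions that set each door's relative X position while keeping Y and Z.
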(event Custom|OpenDoors
  (if (Variables|Default|GetIsClosed)
    (Variables|Default|SetIsClosed false)
    (bind (_direction _leftdoor _rightdoor) (Timeline|Timeline_0 PlayFromStart)
      (:Update
        (CallFunction|MoveLeftDoor _leftdoor)
        (CallFunction|MoveRightDoor _rightdoor)))))

(event Custom|CloseDoors
  (if (not (Variables|Default|GetIsClosed))
    (Variables|Default|SetIsClosed true)
    (bind (_direction _leftdoor _rightdoor) (Timeline|Timeline_0 ReverseFromEnd)
      (:Update
        (CallFunction|MoveLeftDoor _leftdoor)
        (CallFunction|MoveRightDoor _rightdoor)))))

(fn ConstructionScript)

(fn MoveRightDoor
  (params (NewLocation_X :type Float%20%28double-precision%29))
  (bind _floor_door_right (Variables|Default|GetFloor_door_right))
  (bind _relativelocation (Variables|/Script/Engine.SceneComponent|GetRelativeLocation _floor_door_right))
  (Transformation|SetRelativeLocation (Variables|Default|GetFloor_door_right) (Math|Vector|MakeVector NewLocation_X (.y _relativelocation) (.z _relativelocation)) false false))

(fn MoveLeftDoor
  (params (NewLocation_X :type Float%20%28double-precision%29))
  (bind _floor_door_left (Variables|Default|GetFloor_door_left))
  (bind _relativelocation (Variables|/Script/Engine.SceneComponent|GetRelativeLocation _floor_door_left))
  (Transformation|SetRelativeLocation (Variables|Default|GetFloor_door_left) (Math|Vector|MakeVector NewLocation_X (.y _relativelocation) (.z _relativelocation)) false false))