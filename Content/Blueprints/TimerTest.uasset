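; TimerTest is a test Blueprint that exercises a looping timer and shows its activity through printed debug messages.
; BeginPlay starts a one-second looping timer bound to a custom event, which prints on each firing, and stores the handle.
; A Backspace debug key prints a message and clears that timer by its handle.
; Tick separately prints the frame delta time in a different color.
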(event Custom|CustomEvent
  (Development|PrintString "Hello" true true "(R=0.000000,G=0.660000,B=1.000000,A=1.000000)" 1e+01))

(event EventBeginPlay
  (bind _returnvalue (Utilities|Time|SetTimerbyEvent (delegate Custom|CustomEvent) 1.0 true))
  (Variables|Default|SetTimer _returnvalue))

(event EventTick
  (params (DeltaSeconds :type Float%20%28single-precision%29))
  (Development|PrintString (Utilities|String|ToString(Float) DeltaSeconds) true true "(R=0.059148,G=0.087921,B=0.401042,A=1.000000)" 0.1))

(event Input|KeyboardEvents|DebugKeyBackspace
  (params (Key :type Key%20Structure :default "None") (ActionValue :type Input%20Action%20Value%20Structure))
  (:Pressed
    (Development|PrintString "Key" true true "(R=0.364583,G=0.044291,B=0.000000,A=1.000000)")
    (Utilities|Time|ClearandInvalidateTimerbyHandle (Variables|Default|GetTimer))))

(fn ConstructionScript)